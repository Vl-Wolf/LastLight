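; Player character Blueprint that layers animation, aiming and UI hooks onto weapon, inventory and death events.
; Fire and reload events call multicasts, whose handlers forward montages and reload results to the cached ABP_Character instance.
; A reversible timeline drives the ADS alpha, and weapon switches update the matching HUD slot through BP_PlayerController.
; Death unpossesses the controller; BeginPlay also prints current health as debug output.
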(event OnSwitchWeapon(InventoryComponent)
  (params (WeaponId :type Name :default "None") (WeaponAdditionalInfo :type Additional%20Weapon%20Info%20Structure) (NewCurrentIndexWeapon :type Integer))
  (bind _asbp_player_controller (Utilities|Casting|CastToBP_PlayerController (Pawn|GetController)))
  (Utilities|IsValid (Variables|/Game/Blueprint/Game/BP_PlayerController.BP_PlayerController_C|GetInGameWidget _asbp_player_controller)
    (:Is%20Valid
      (bind _asbpw_weapon_slots (Utilities|Casting|CastToBPW_WeaponSlots (Class|PanelWidget|GetChildat (Variables|/Game/Widget/Inventory/BPW_InventoryStatsWidget.BPW_InventoryStatsWidget_C|GetWeaponSlots (Variables|/Game/Widget/BPW_InGameWidget.BPW_InGameWidget_C|GetBPW_InventoryStatsWidget (Variables|/Game/Blueprint/Game/BP_PlayerController.BP_PlayerController_C|GetInGameWidget _asbp_player_controller))) NewCurrentIndexWeapon)))
      (Default|UpdateInfo _asbpw_weapon_slots WeaponId (Utilities|Struct|BreakAdditionalWeaponInfo WeaponAdditionalInfo)))))

(event Custom|ReloadAnimEnd_Multicast
  (params (bIsSuccess :type Boolean))
  (Default|ReloadingEnd (Variables|Default|GetAnimInstance) bIsSuccess))

(event Custom|FireAnimStart_Multicast
  (params (MontageToPlay :type Anim%20Montage%20Object%20Reference))
  (Default|Firing (Variables|Default|GetAnimInstance) MontageToPlay))

(event Custom|ReloadAnimStart_Multicast
  (params (MontageToPlay :type Anim%20Montage%20Object%20Reference))
  (Default|Reloading (Variables|Default|GetAnimInstance) MontageToPlay))

(event EventWeaponFireBP
  (params (Anim :type Anim%20Montage%20Object%20Reference))
  (CallFunction|FireAnimStartMulticast Anim))

(event EventBeginPlay
  (bind _asabp_character (Utilities|Casting|CastToABP_Character (Components|SkeletalMesh|GetAnimInstance (Variables|Character|GetMesh))))
  (Variables|Default|SetAnimInstance _asabp_character)
  (bind _returnvalue (Class|LastLightHealthComponent|GetCurrentHealth (Variables|Default|GetHealthComponent)))
  (Development|PrintString (Utilities|String|ToString(Float) _returnvalue)))

(event EventToggleADSBP
  (params (toggle :type Boolean))
  (if toggle
    (bind _adsalpha (Timeline|ADS_Timeline Play)
      (:Update
        (Variables|Default|SetADSValue _adsalpha)))
    (else
      (Timeline|ADS_Timeline Reverse))))

(event EventWeaponReloadStartBP
  (params (Anim :type Anim%20Montage%20Object%20Reference))
  (CallFunction|ReloadAnimStartMulticast Anim))

(event EventWeaponReloadEndBP
  (params (bIsSuccess :type Boolean))
  (CallFunction|ReloadAnimEndMulticast bIsSuccess))

(event EventCharacterDeadBP
  (bind _asbp_player_controller (Utilities|Casting|CastToBP_PlayerController (Pawn|GetController)))
  (bind _output_get (Variables|Default|SetAs%20BP%20Player%20Controller _asbp_player_controller))
  (Pawn|UnPossess _output_get))

(event EventTick
  (params (DeltaSeconds :type Float%20%28single-precision%29)))

(fn ConstructionScript)