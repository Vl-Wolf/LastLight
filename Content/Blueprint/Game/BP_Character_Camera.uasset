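; BP_Character_Camera is a player camera manager that drives BP_Character's first-person view while a weapon is held, including aim-down-sights.
; BlueprintUpdateCamera follows control rotation, blending location from the character camera toward the weapon's IronSight socket axis and narrowing FOV by ADSValue.
; Each tick, WeaponSway eases SwayOffset toward zero, then toward SwayADS or SwayIndle by ADS state.
; The camera update adds that offset, rotated into view space.
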(event Custom|WeaponSway
  (Utilities|IsValid (Variables|Default|GetCharacter)
    (:Is%20Valid
      (Variables|Default|SetSwayOffset (Math|Interpolation|VInterpTo (Variables|Default|GetSwayOffset) "0, 0, 0" (Utilities|Time|GetWorldDeltaSeconds) 6.0))
      (Variables|Default|SetSwayOffset (Math|Interpolation|VInterpTo (Variables|Default|GetSwayOffset) (select (Class|LastLightCharacter|GetADSEnabled (Variables|Default|GetCharacter)) (Utilities|SwayADS) (Utilities|SwayIndle)) (Utilities|Time|GetWorldDeltaSeconds) 5.0)))))

(event EventTick
  (params (DeltaSeconds :type Float%20%28single-precision%29))
  (CallFunction|WeaponSway))

(fn ConstructionScript)

(fn BlueprintUpdateCamera
  (params (CameraTarget :type Actor%20Object%20Reference))
  (bind _asbp_character (Utilities|Casting|CastToBP_Character CameraTarget))
  (bind _output_get (Variables|Default|SetCharacter _asbp_character))
  (Utilities|IsValid _output_get
    (:Is%20Valid
      (Utilities|IsValid (Class|LastLightCharacter|GetCurrentWeapon (Variables|Default|GetCharacter))
        (:Is%20Valid
          (Variables|Default|SetFinalCameraRotation (Pawn|GetControlRotation (Variables|Default|GetCharacter) :!class /Script/Engine.Pawn))
          (Variables|Default|SetFinalCameraLocation (+ (Math|Vector|RotateVector (Variables|Default|GetSwayOffset) (Variables|Default|GetFinalCameraRotation)) (Math|Vector|Lerp(Vector) (Transformation|GetWorldLocation (Variables|/Script/LastLight.LastLightCharacter|GetCamera (Variables|Default|GetCharacter))) (- (.Location (Math|Transform|BreakTransform (Transformation|GetSocketTransform (Variables|/Script/LastLight.WeaponDefault|GetSkeletalMeshWeapon (Class|LastLightCharacter|GetCurrentWeapon (Variables|Default|GetCharacter))) "IronSight" "RTS_World"))) (* (Math|Vector|GetForwardVector (.Rotation (Math|Transform|BreakTransform (Transformation|GetSocketTransform (Variables|/Script/LastLight.WeaponDefault|GetSkeletalMeshWeapon (Class|LastLightCharacter|GetCurrentWeapon (Variables|Default|GetCharacter))) "IronSight" "RTS_World")))) (* (Math|Vector|DotProduct (Math|Vector|Normalize (- (.Location (Math|Transform|BreakTransform (Transformation|GetSocketTransform (Variables|/Script/LastLight.WeaponDefault|GetSkeletalMeshWeapon (Class|LastLightCharacter|GetCurrentWeapon (Variables|Default|GetCharacter))) "IronSight" "RTS_World"))) (Transformation|GetWorldLocation (Variables|/Script/LastLight.LastLightCharacter|GetCamera (Variables|Default|GetCharacter)))) 0.0) (Math|Vector|GetForwardVector (.Rotation (Math|Transform|BreakTransform (Transformation|GetSocketTransform (Variables|/Script/LastLight.WeaponDefault|GetSkeletalMeshWeapon (Class|LastLightCharacter|GetCurrentWeapon (Variables|Default|GetCharacter))) "IronSight" "RTS_World"))))) (/ (Math|Vector|VectorLength (- (.Location (Math|Transform|BreakTransform (Transformation|GetSocketTransform (Variables|/Script/LastLight.WeaponDefault|GetSkeletalMeshWeapon (Class|LastLightCharacter|GetCurrentWeapon (Variables|Default|GetCharacter))) "IronSight" "RTS_World"))) (Transformation|GetWorldLocation (Variables|/Script/LastLight.LastLightCharacter|GetCamera (Variables|Default|GetCharacter))))) 1e+02)))) (Variables|/Game/Blueprint/Character/BP_Character.BP_Character_C|GetADSValue (Variables|Default|GetCharacter)))))
          (return (Variables|Default|GetFinalCameraLocation) (Variables|Default|GetFinalCameraRotation) (Math|Float|Lerp 9e+01 8e+01 (Variables|/Game/Blueprint/Character/BP_Character.BP_Character_C|GetADSValue (Variables|Default|GetCharacter))) true))))))