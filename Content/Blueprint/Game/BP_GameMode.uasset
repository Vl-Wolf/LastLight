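; BP_GameMode is a game mode that moves a dead player into spectating a surviving character.
; TryTorespawnPlayerAtSpectator searches the Controllers array for the first pawn that is a living BP_Character.
; It spawns a BP_PlayerSpectator at that character's location with it as TargetPawn, then has the dead player's controller possess the spectator.
; When no valid target exists it only prints "EndGame".
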(event EventBeginPlay)

(event EventTick
  (params (DeltaSeconds :type Float%20%28single-precision%29)))

(fn ConstructionScript)

(fn TryTorespawnPlayeratSpectator
  (params (PlayerControllerDead :type BP%20Player%20Controller%20Object%20Reference))
  (bind _array_element (Utilities|Array|ForEachLoopwithBreak (Variables|Default|GetControllers) :!label _label)
    (:LoopBody
      (bind _asbp_character (Utilities|Casting|CastToBP_Character (Pawn|GetControlledPawn _array_element)))
      (if (Class|LastLightCharacter|GetIsAlive _asbp_character)
        (LocalVariables|SetTargetForSpectator _asbp_character)
        (goto _label Break)))
    (:Completed
      (Utilities|IsValid (LocalVariables|GetTargetForSpectator)
        (:Is%20Valid
          (bind _returnvalue (Game|SpawnActorfromClass "/Game/Blueprint/Game/BP_PlayerSpectator.BP_PlayerSpectator_C" (Math|Conversions|ToTransform(Vector) (Transformation|GetActorLocation (LocalVariables|GetTargetForSpectator))) "AlwaysSpawn" 0 (LocalVariables|GetTargetForSpectator) 0))
          (Pawn|Possess PlayerControllerDead _returnvalue))
        (:Is%20Not%20Valid
          (Development|PrintString "EndGame"))))))