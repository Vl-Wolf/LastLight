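; Player controller that creates the in-game HUD and keeps its inventory and health bar widgets bound to the player's BP_Character.
; BeginPlay builds the HUD for the local player and initializes it from the character's inventory component.
; On possess, weapon and ammo slots stored in BP_PlayerState initialize the character's server-side inventory and refresh the HUD.
; On unpossess, the inventory and health widgets are unbound from the character.
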(event Custom|InitWidget
  (params (NewWeaponSlotsInfo :type Array%20of%20Weapon%20Slot%20Structures) (NewAmmoSlotsInfo :type Array%20of%20Ammo%20Slot%20Structures))
  (bind _ingamewidget (Variables|Default|GetInGameWidget))
  (bind _bpw_inventorystatswidget (Variables|/Game/Widget/BPW_InGameWidget.BPW_InGameWidget_C|GetBPW_InventoryStatsWidget _ingamewidget))
  (Utilities|IsValid _ingamewidget
    (:Is%20Valid
      (bind _asbp_character (Utilities|Casting|CastToBP_Character (Game|Player|GetPlayerPawn 0)))
      (Default|BindInventoryEvents _bpw_inventorystatswidget _asbp_character)
      (Default|InitInventorySlots _bpw_inventorystatswidget NewWeaponSlotsInfo NewAmmoSlotsInfo)
      (Default|InitWidget (Variables|/Game/Widget/BPW_InGameWidget.BPW_InGameWidget_C|GetBPW_HealthBar _ingamewidget) _asbp_character))))

(event Custom|UnbindWidgetEvents
  (params (Object :type Object%20Object%20Reference))
  (CallFunction|UnbindWidgets Object))

(event EventBeginPlay
  (Networking|SwitchHasAuthority
    (:Authority
      (if (Pawn|IsLocalPlayerController)
        (bind _returnvalue (UserInterface|CreateWidget "/Game/Widget/BPW_InGameWidget.BPW_InGameWidget_C" self :!label _label))
        (bind _output_get (Variables|Default|SetInGameWidget _returnvalue))
        (UserInterface|Viewport|AddtoViewport _output_get 0)
        (bind _asbp_character (Utilities|Casting|CastToBP_Character (Game|Player|GetPlayerPawn 0)))
        (Default|BindInventoryEvents (Variables|/Game/Widget/BPW_InGameWidget.BPW_InGameWidget_C|GetBPW_InventoryStatsWidget _output_get) _asbp_character)
        (Default|InitInventorySlots (Variables|/Game/Widget/BPW_InGameWidget.BPW_InGameWidget_C|GetBPW_InventoryStatsWidget _output_get) (Variables|/Script/LastLight.LastLightInventoryComponent|GetWeaponSlots (Variables|/Script/LastLight.LastLightCharacter|GetInventoryComponent _asbp_character)) (Variables|/Script/LastLight.LastLightInventoryComponent|GetAmmoSlots (Variables|/Script/LastLight.LastLightCharacter|GetInventoryComponent _asbp_character)))
        (Default|InitWidget (Variables|/Game/Widget/BPW_InGameWidget.BPW_InGameWidget_C|GetBPW_HealthBar _output_get) _asbp_character)))
    (:Remote
      (goto _label))))

(event EventPossess
  (params (PossessedPawn :type Pawn%20Object%20Reference))
  (bind _asbp_character (Utilities|Casting|CastToBP_Character PossessedPawn))
  (bind _asbp_player_state (Utilities|Casting|CastToBP_PlayerState (Variables|GetPlayerState)))
  (Class|LastLightInventoryComponent|InitInventoryonServer (Variables|/Script/LastLight.LastLightCharacter|GetInventoryComponent _asbp_character) (Variables|/Game/Blueprint/Game/BP_PlayerState.BP_PlayerState_C|GetWeaponSlots _asbp_player_state) (Variables|/Game/Blueprint/Game/BP_PlayerState.BP_PlayerState_C|GetAmmoSlots _asbp_player_state))
  (CallFunction|InitWidget (Variables|/Game/Blueprint/Game/BP_PlayerState.BP_PlayerState_C|GetWeaponSlots _asbp_player_state) (Variables|/Game/Blueprint/Game/BP_PlayerState.BP_PlayerState_C|GetAmmoSlots _asbp_player_state)))

(event EventUnPossess
  (params (UnpossessedPawn :type Pawn%20Object%20Reference))
  (CallFunction|UnbindWidgetEvents UnpossessedPawn))

(fn ConstructionScript)

(fn UnbindWidgets
  (params (Target :type Object%20Object%20Reference))
  (bind _ingamewidget (Variables|Default|GetInGameWidget))
  (Utilities|IsValid Target
    (:Is%20Valid
      (LocalVariables|SetmyTarget Target))
    (:Is%20Not%20Valid
      (LocalVariables|SetmyTarget (Pawn|GetControlledPawn))))
  (bind _asbp_character (Utilities|Casting|CastToBP_Character (LocalVariables|GetmyTarget)))
  (Default|UnbindAllEvents (Variables|/Game/Widget/BPW_InGameWidget.BPW_InGameWidget_C|GetBPW_InventoryStatsWidget _ingamewidget) _asbp_character)
  (Default|UnBindWidget (Variables|/Game/Widget/BPW_InGameWidget.BPW_InGameWidget_C|GetBPW_HealthBar _ingamewidget)))