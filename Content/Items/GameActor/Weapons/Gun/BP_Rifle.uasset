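; BP_Rifle is a rifle weapon Blueprint with a ShootLocation component, and it has no active logic in these graphs.
; BeginPlay and the construction script are empty.
; Each graph holds an unconnected debug line trace that would run forward from ShootLocation on the Visibility channel, but it never executes.
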(event EventBeginPlay)

(fn ConstructionScript)